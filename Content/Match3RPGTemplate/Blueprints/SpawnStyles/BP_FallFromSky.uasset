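; Spawn style for the Match3 RPG template that makes a unit drop from the sky onto its spawn location.
; It hides the UI, raises the unit above the spawn point, starts an animation, and lerps it down with a timeline.
; On landing it switches animation, plays a world camera shake at the unit, shows the UI, and signals that spawning has finished.
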(event `self.Spawn`
  (bind _spawnlocation (`self.spawnLocation`))
  (bind (_returnvalue_location _returnvalue_rotation _returnvalue_scale) (`KismetMathLibrary.BreakTransform` (`self.GetTransform` _spawnlocation)))
  ;[1 1 1] Make the unit fall from sky
  (`self.HideUI`)
  (bind _output_get (set `self.startLocation` (+ _returnvalue_location (* (0.0 0.0 750.0) (`self.GetActorUpVector` _spawnlocation)))))
  (`self.K2_SetActorTransform` (`self.unit`) (`KismetMathLibrary.MakeTransform` _output_get _returnvalue_rotation _returnvalue_scale) false false)
  (`/Game/Match3RPGTemplate/Blueprints/Units/BP_UnitBase.PlayAnimation` (`self.unit`) "NewEnumerator2")
  (bind (_direction _alpha) (`Timeline|MoveOverTime` :!via `PlayFromStart`)
    (:`Update`
      (`self.K2_SetActorLocation` (`self.unit`) (`KismetMathLibrary.VLerp` (`self.startLocation`) (`self.K2_GetActorLocation` (`self.spawnLocation`)) _alpha) false false))
    (:`Finished`
      (`self.OnLanded`))))

(event `OnLanded`
  (bind _unit (`self.unit`))
  ;[1 1 1] Shake camera on landing
  (`/Game/Match3RPGTemplate/Blueprints/Units/BP_UnitBase.PlayAnimation` _unit "NewEnumerator0")
  (`GameplayStatics.PlayWorldCameraShake` "/Game/Match3RPGTemplate/Blueprints/SpawnStyles/BP_FallFromSkyShake.BP_FallFromSkyShake_C" (`self.K2_GetActorLocation` _unit) 5000.0 10000.0)
  (`self.ShowUI`)
  (`self.OnSpawnFinished`))

(fn `UserConstructionScript`
  (`parent.UserConstructionScript`))