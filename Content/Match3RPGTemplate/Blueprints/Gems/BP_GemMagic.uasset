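; BP_GemMagic is a Match-3 RPG gem that spends player mana to attack the current enemy when matched.
; While matching, it previews damage through the BattleManager and flags a potential kill.
; On match it reduces mana, moves the player to the enemy and times the hit to the animation, dealing half damage if remaining mana is below a threshold.
; The player then moves back and the turn ends.
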(event `self.UpdateMatchingDetails`
  (params (matchingDetailsUI :type "/Game/Match3RPGTemplate/Blueprints/UI/BP_MatchingDetailsUI Object Reference") (matchedGemAmount :type Integer))
  ;[1 1 1] Show gem information when matching
  (bind _playerdamage (`/Game/Match3RPGTemplate/Blueprints/BP_BattleManager.GetPlayerDamage` (`self.battleManager`) matchedGemAmount))
  (if (== 0 _playerdamage)
    (`/Game/Match3RPGTemplate/Blueprints/UI/BP_MatchingDetailsUI.UpdateMatchingDetails` matchingDetailsUI "Damage" (`KismetTextLibrary.Conv_IntToText` _playerdamage) "" (struct :`R` 0.171875 :`G` 0.171875 :`B` 0.171875 :`A` 1.0))
    (else
      (bind _returnvalue (and (> matchedGemAmount 2) (>= _playerdamage (`/Game/Match3RPGTemplate/Blueprints/Units/BP_UnitBase.currentHP` (`/Game/Match3RPGTemplate/Blueprints/BP_BattleManager.currentEnemy` (`self.battleManager`))))))
      (`/Game/Match3RPGTemplate/Blueprints/UI/BP_MatchingDetailsUI.UpdateMatchingDetails` matchingDetailsUI "Damage" (`KismetTextLibrary.Conv_IntToText` _playerdamage) (select `bool` _returnvalue :`true` "-KILL-" :!type "Text") (select `bool` _returnvalue :`false` (struct :`R` 1.0 :`G` 1.0 :`B` 1.0 :`A` 1.0) :`true` (struct :`R` 1.0 :`A` 1.0) :!type "LinearColor Structure")))))

(event `self.OnMatch`
  (params (matchedGemAmount :type Integer))
  ;[1 1 1] Move player next to enemy on match
  (bind _output_get (set `self.matchedGemAmount` matchedGemAmount))
  (`/Game/Match3RPGTemplate/Blueprints/Units/Player/BP_PlayerBase.ReduceMana` (`/Game/Match3RPGTemplate/Blueprints/BP_BattleManager.player` (`self.battleManager`)) _output_get)
  (`self.PlayerMove` (delegate `OnMovedToEnemyHandler`)))

(event `OnMovedToEnemyHandler`
  ;[1 1 1] Move player next to enemy on match
  (`self.PlayAttack`))

(event `OnPlayerMovedBackHandler`
  ;[1 1 1] Player attacks
  (`self.OnPlayersTurnEnded`))

(event `PlayAttack`
  (bind _player (`/Game/Match3RPGTemplate/Blueprints/BP_BattleManager.player` (`self.battleManager`)))
  (bind _player_2 (`/Game/Match3RPGTemplate/Blueprints/BP_BattleManager.player` (`self.battleManager`)))
  (bind _animationhitdelay (`/Game/Match3RPGTemplate/Blueprints/Units/BP_UnitBase.animationHitDelay` _player_2))
  (bind _animationhitdelay_2 (`/Game/Match3RPGTemplate/Blueprints/Units/BP_UnitBase.animationHitDelay` _player))
  (if (<= 10 (`/Game/Match3RPGTemplate/Blueprints/Units/Player/BP_PlayerBase.currentMana` (`/Game/Match3RPGTemplate/Blueprints/BP_BattleManager.player` (`self.battleManager`))))
    ;[1 1 1] Player attacks
    (bind _animationlength (`/Game/Match3RPGTemplate/Blueprints/Units/BP_UnitBase.PlayAnimation` _player_2 "NewEnumerator3"))
    (`KismetSystemLibrary.Delay` _animationhitdelay)
    (`/Game/Match3RPGTemplate/Blueprints/BP_BattleManager.PlayerDoDamage` (`self.battleManager`) (`self.matchedGemAmount`))
    (bind _returnvalue (- _animationlength _animationhitdelay))
    (`KismetSystemLibrary.Delay` (select `bool` (> _returnvalue 0.0) :`true` _returnvalue))
    (`self.PlayerMoveBack` (delegate `OnPlayerMovedBackHandler`))
    (else
      ;[1 1 1] Player attacks
      (bind _animationlength_2 (`/Game/Match3RPGTemplate/Blueprints/Units/BP_UnitBase.PlayAnimation` _player "NewEnumerator3"))
      (`KismetSystemLibrary.Delay` _animationhitdelay_2)
      (`/Game/Match3RPGTemplate/Blueprints/BP_BattleManager.PlayerDoHalfDamage` (`self.battleManager`) (`self.matchedGemAmount`))
      (bind _returnvalue_2 (- _animationlength_2 _animationhitdelay_2))
      (`KismetSystemLibrary.Delay` (select `bool` (> _returnvalue_2 0.0) :`true` _returnvalue_2))
      (`self.PlayerMoveBack` (delegate `CustomEvent_1`)))))

(event `CustomEvent_1`
  ;[1 1 1] Player attacks
  (`self.OnPlayersTurnEnded`))

(fn `UserConstructionScript`
  (`parent.UserConstructionScript`))