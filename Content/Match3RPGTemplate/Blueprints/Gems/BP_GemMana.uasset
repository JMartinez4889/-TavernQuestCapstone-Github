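; BP_GemMana is the mana gem in the match-3 RPG battle, a child gem Blueprint that restores the player's mana when matched.
; While matching, it fills the matching details UI with a blue "Mana" title, the gain amount, and a "-FULL-" note when that gain would reach the player's max mana.
; On match, it adds the matched gem count to the player's mana through the BattleManager, then ends the player's turn.
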(event `self.UpdateMatchingDetails`
  (params (matchingDetailsUI :type "/Game/Match3RPGTemplate/Blueprints/UI/BP_MatchingDetailsUI Object Reference") (matchedGemAmount :type Integer))
  (bind _player (`/Game/Match3RPGTemplate/Blueprints/BP_BattleManager.player` (`self.battleManager`)))
  ;[1 1 1] Show gem information when matching
  (`/Game/Match3RPGTemplate/Blueprints/UI/BP_MatchingDetailsUI.UpdateMatchingDetails` matchingDetailsUI "Mana" (`|FormatText` "+{Amount}" (`KismetTextLibrary.Conv_IntToText` matchedGemAmount)) (select `bool` (>= (+ matchedGemAmount (`/Game/Match3RPGTemplate/Blueprints/Units/Player/BP_PlayerBase.currentMana` _player)) (`/Game/Match3RPGTemplate/Blueprints/Units/Player/BP_PlayerBase.maxMana` _player)) :`true` "-FULL-" :!type "Text") (struct :`G` 0.5 :`B` 1.0 :`A` 1.0)))

(event `self.OnMatch`
  (params (matchedGemAmount :type Integer))
  ;[1 1 1] Increase mana on match
  (`/Game/Match3RPGTemplate/Blueprints/Units/Player/BP_PlayerBase.IncreaseMana` (`/Game/Match3RPGTemplate/Blueprints/BP_BattleManager.player` (`self.battleManager`)) matchedGemAmount)
  (`self.OnPlayersTurnEnded`))

(fn `UserConstructionScript`
  (`parent.UserConstructionScript`))