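; Shield gem for the match-3 RPG battle, letting matched gems factor into the damage the player takes from the enemy.
; While matching, it asks BattleManager for the resulting enemy damage and previews it as a green block or red damage value, with a warning if lethal.
; On match, if the enemy has attack power, it plays a player animation and stores the gem count on BattleManager.
; It always ends the player's turn.
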(event `self.UpdateMatchingDetails`
  (params (matchingDetailsUI :type "/Game/Match3RPGTemplate/Blueprints/UI/BP_MatchingDetailsUI Object Reference") (matchedGemAmount :type Integer))
  ;[1 1 1] Show gem information when matching
  (bind _enemydamage (`/Game/Match3RPGTemplate/Blueprints/BP_BattleManager.GetEnemyDamage` (`self.battleManager`) matchedGemAmount))
  (bind _returnvalue (== _enemydamage 0))
  (`/Game/Match3RPGTemplate/Blueprints/UI/BP_MatchingDetailsUI.UpdateMatchingDetails` matchingDetailsUI (select `bool` _returnvalue :`false` "Shield" :`true` "-BLOCK-" :!type "Text") (select `bool` _returnvalue :`false` (`|FormatText` "-{damage}" _enemydamage)) (select `bool` (>= _enemydamage (`/Game/Match3RPGTemplate/Blueprints/Units/BP_UnitBase.currentHP` (`/Game/Match3RPGTemplate/Blueprints/BP_BattleManager.player` (`self.battleManager`)))) :`true` "-YOU DIE-" :!type "Text") (select `bool` _returnvalue :`false` (struct :`R` 1.0 :`A` 1.0) :`true` (struct :`G` 1.0 :`A` 1.0) :!type "LinearColor Structure")))

(event `self.OnMatch`
  (params (matchedGemAmount :type Integer))
  ;[1 1 1] Set matched shield gem amount
  (bind _enemyattackpower (`/Game/Match3RPGTemplate/Blueprints/BP_BattleManager.GetCurrentEnemyAttackPower` (`self.battleManager`)))
  (if (== _enemyattackpower 0)
    (`self.OnPlayersTurnEnded`)
    (else
      (`/Game/Match3RPGTemplate/Blueprints/Units/BP_UnitBase.PlayAnimation` (`/Game/Match3RPGTemplate/Blueprints/BP_BattleManager.player` (`self.battleManager`)) "NewEnumerator7")
      (set `/Game/Match3RPGTemplate/Blueprints/BP_BattleManager.matchedShieldGemAmount` matchedGemAmount (`self.battleManager`))
      (`self.OnPlayersTurnEnded`))))

(fn `UserConstructionScript`
  (`parent.UserConstructionScript`))