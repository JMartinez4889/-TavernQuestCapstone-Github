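; Battle manager for a match-3 RPG that runs one stage fight: it spawns the stage and player, then enemies from a list one after another.
; Matched gem amounts, equipped gear and unit stats drive damage, with floating text and death handling.
; Player skills from character and gear use mana and cooldowns; enemies work through a refilled queue of weighted-random skills on countdowns.
; Events report each battle step to listeners.
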(event `Initialize`
  (params (player :type "/Game/Match3RPGTemplate/Blueprints/Units/Player/BP_PlayerBase Class Reference") (stageData :type "/Game/Match3RPGTemplate/Blueprints/StageData Structure"))
  (bind (_stage _enemylist) (break `/Game/Match3RPGTemplate/Blueprints/StageData` stageData))
  ;[1 1 1] Initialize
  (set `self.match3RPGPlayerController` (cast `/Game/Match3RPGTemplate/Blueprints/BP_Match3RPGPlayerController` (`GameplayStatics.GetPlayerController` 0) :!pure true))
  (`self.SpawnStage` _stage)
  (`self.SpawnPlayer` player)
  (set `self.enemyList` _enemylist)
  (set `self.currentEnemyIndex` 0))

(event `SpawnStage`
  (params (stage :type "/Game/Match3RPGTemplate/Blueprints/Stages/BP_StageBase Class Reference"))
  ;[1 1 1] Spawn Stage
  (if (`KismetSystemLibrary.IsValidClass` stage)
    (bind _returnvalue (`|SpawnActorFromClass` stage (`KismetMathLibrary.MakeTransform` (0.0 0.0 0.0)) "Undefined" "OverrideRootScale" null null))
    (bind _output_get (set `self.stage` _returnvalue))
    (`PlayerController.SetViewTargetWithBlend` (`self.match3RPGPlayerController`) _output_get 0.0 "VTBlend_Linear" 0.0 false)
    (else
      (`KismetSystemLibrary.PrintString` "Stage is not set !" true true (struct :`R` 1.0 :`A` 1.0) 5.0))))

(event `SpawnPlayer`
  (params (player :type "/Game/Match3RPGTemplate/Blueprints/Units/Player/BP_PlayerBase Class Reference"))
  ;[1 1 1] Spawn Player
  (if (`KismetSystemLibrary.IsValidClass` player)
    (bind _returnvalue (`|SpawnActorFromClass` player (`KismetMathLibrary.MakeTransform` (9999999.0 9999999.0 9999999.0)) "Undefined" "OverrideRootScale" null null))
    (bind _output_get (set `self.player` _returnvalue))
    (add `/Game/Match3RPGTemplate/Blueprints/Units/BP_UnitBase.OnUnitSpawned` _output_get (delegate `OnPlayerSpawnedHandler`))
    (`self.CreatePlayerSkills`)
    (`/Game/Match3RPGTemplate/Blueprints/Units/BP_UnitBase.Spawn` (`self.player`) (cast `/Game/Match3RPGTemplate/Blueprints/BP_UnitSpawnLocation` (`ChildActorComponent.ChildActor` (`/Game/Match3RPGTemplate/Blueprints/Stages/BP_StageBase.PlayerSpawnLocation` (`self.stage`))) :!pure true))
    (else
      (`KismetSystemLibrary.PrintString` "Player is not set !" true true (struct :`R` 1.0 :`A` 1.0) 5.0))))

(event `OnPlayerSpawnedHandler`
  ;[1 1 1] Spawn Player
  (`self.OnBattleManagerInitialized`))

(event `SpawnEnemy`
  ;[1 1 1] Spawn Enemy
  (if (> (`KismetArrayLibrary.Array_Length` (`self.enemyList`)) 0)
    (bind _returnvalue (`|SpawnActorFromClass` (`|GetArrayItem` (`self.enemyList`) (`self.currentEnemyIndex`)) (`KismetMathLibrary.MakeTransform` (9999999.0 9999999.0 9999999.0)) "Undefined" "OverrideRootScale" null null))
    (bind _output_get (set `self.currentEnemy` _returnvalue))
    (add `/Game/Match3RPGTemplate/Blueprints/Units/BP_UnitBase.OnUnitSpawned` _output_get (delegate `OnEnemySpawnedHandler`))
    (`self.CreateEnemySkill` 5)
    (`/Game/Match3RPGTemplate/Blueprints/Units/BP_UnitBase.Spawn` (`self.currentEnemy`) (cast `/Game/Match3RPGTemplate/Blueprints/BP_UnitSpawnLocation` (`ChildActorComponent.ChildActor` (`/Game/Match3RPGTemplate/Blueprints/Stages/BP_StageBase.EnemySpawnLocation` (`self.stage`))) :!pure true))
    (else
      (`KismetSystemLibrary.PrintString` "Enemy is not set !" true true (struct :`R` 1.0 :`A` 1.0) 5.0))))

(event `OnEnemySpawnedHandler`
  ;[1 1 1] Spawn Enemy
  (`self.OnEnemySpawned`))

(event `CreatePlayerSkills`
  ;[1 1 1] Spawn Player skills
  (bind _playerskills (`self.GetPlayerSkills`))
  (for _array_element _playerskills
    (bind _returnvalue (`|SpawnActorFromClass` _array_element (`KismetMathLibrary.MakeTransform` (0.0 0.0 0.0)) "Undefined" "OverrideRootScale" null self null))
    (`KismetArrayLibrary.Array_Add` (`self.playerSkills`) _returnvalue)
    (add `/Game/Match3RPGTemplate/Blueprints/Skills/BP_SkillBase.OnSkillUsed` _returnvalue (delegate `OnPlayerSkillUsedHandler`))))

(event `OnPlayerSkillUsedHandler`
  ;[1 1 1] Spawn Player skills
  (`self.OnPlayerSkillUsed`))

(event `CreateEnemySkill`
  (params (amount :type Integer))
  ;[1 1 1] Spawn Enemy Skills
  (for _ (range 1 (+ amount 1))
    (bind _enemyskill (`self.GetEnemySkillBasedOnWeight`))
    (bind _returnvalue (`|SpawnActorFromClass` _enemyskill (`KismetMathLibrary.MakeTransform` (0.0 0.0 0.0)) "Undefined" "OverrideRootScale" null self null))
    (`KismetArrayLibrary.Array_Add` (`self.EnemySkills`) _returnvalue)))

(event `self.ReceiveTick`
  (params (DeltaSeconds :type "Float (single-precision)"))
  ;[1 1 1] Save delta seconds
  (set `self.deltaSeconds` DeltaSeconds))

(event `UnitMove`
  (params (moveAnimation :type "/Game/Match3RPGTemplate/Blueprints/Units/AnimationType Enum" :default "NewEnumerator0") (moveSpeed :type "Float (double-precision)") (fromLocation :type "Vector Structure") (toLocation :type "Vector Structure") (unit :type "/Game/Match3RPGTemplate/Blueprints/Units/BP_UnitBase Object Reference"))
  ;[1 1 1] Moves a unit to given location
  (`/Game/Match3RPGTemplate/Blueprints/Units/BP_UnitBase.PlayAnimation` unit moveAnimation)
  (`TimelineComponent.SetPlayRate` (`self.PlayerMoveOverTime`) (/ moveSpeed (`KismetMathLibrary.VSize` (- fromLocation toLocation))))
  (`Timeline|PlayerMoveOverTime` :!via `PlayFromStart`
    (:`Update`
      (`self.K2_SetActorLocation` unit (`KismetMathLibrary.VInterpTo_Constant` (`self.K2_GetActorLocation` unit) toLocation (`self.deltaSeconds`) moveSpeed) false false))
    (:`Finished`
      (`/Game/Match3RPGTemplate/Blueprints/Units/BP_UnitBase.PlayAnimation` unit "NewEnumerator0")
      (`self.OnUnitMoved`)
      (clear `self.OnUnitMoved`))))

(event `PlayerDoHalfDamage`
  (params (matchedGemAmount :type Integer))
  ;[1 1 1] Player unit does half damage
  (bind _playerdamage (`self.GetPlayerDamage` matchedGemAmount))
  (bind _returnvalue (/ _playerdamage 2))
  (`/Game/Match3RPGTemplate/Blueprints/Units/BP_UnitBase.TakeDamage` (`self.currentEnemy`) _returnvalue)
  (`|SpawnActorFromClass` "/Game/Match3RPGTemplate/Blueprints/BP_DamageText.BP_DamageText_C" (`self.GetTransform` (`self.currentEnemy`)) "Undefined" "OverrideRootScale" null _returnvalue (struct :`R` 1.0 :`G` 1.0 :`B` 1.0 :`A` 1.0) null)
  (bind _isunitdead (`/Game/Match3RPGTemplate/Blueprints/Units/BP_UnitBase.IsUnitDead` (`self.currentEnemy`)))
  (if _isunitdead
    (`self.KillEnemy`)
    (else
      (`/Game/Match3RPGTemplate/Blueprints/Units/BP_UnitBase.PlayAnimation` (`self.currentEnemy`) "NewEnumerator4"))))

(event `PlayerDoDamage`
  (params (matchedGemAmount :type Integer))
  ;[1 1 1] Player unit does damage
  (bind _playerdamage (`self.GetPlayerDamage` matchedGemAmount))
  (`/Game/Match3RPGTemplate/Blueprints/Units/BP_UnitBase.TakeDamage` (`self.currentEnemy`) _playerdamage)
  (`|SpawnActorFromClass` "/Game/Match3RPGTemplate/Blueprints/BP_DamageText.BP_DamageText_C" (`self.GetTransform` (`self.currentEnemy`)) "Undefined" "OverrideRootScale" null _playerdamage (struct :`R` 1.0 :`G` 1.0 :`B` 1.0 :`A` 1.0) null)
  (bind _isunitdead (`/Game/Match3RPGTemplate/Blueprints/Units/BP_UnitBase.IsUnitDead` (`self.currentEnemy`)))
  (if _isunitdead
    (`self.KillEnemy`)
    (else
      (`/Game/Match3RPGTemplate/Blueprints/Units/BP_UnitBase.PlayAnimation` (`self.currentEnemy`) "NewEnumerator4"))))

(event `EnemyDoDamage`
  (bind _player (`self.player`))
  ;[1 1 1] Enemy does damage
  (bind _enemydamage (`self.GetEnemyDamage` (`KismetMathLibrary.SelectInt` (`self.matchedShieldGemAmount`) (`/Game/Match3RPGTemplate/Blueprints/Units/Player/BP_PlayerBase.OverHealth` _player) (<= (`/Game/Match3RPGTemplate/Blueprints/Units/BP_UnitBase.currentOverhealth` _player) 0))))
  (`/Game/Match3RPGTemplate/Blueprints/Units/BP_UnitBase.TakeDamage` (`self.player`) _enemydamage)
  (bind _returnvalue (== _enemydamage 0))
  (`|SpawnActorFromClass` "/Game/Match3RPGTemplate/Blueprints/BP_DamageText.BP_DamageText_C" (`self.GetTransform` (`self.player`)) "Undefined" "OverrideRootScale" null _enemydamage (select `bool` _returnvalue :`false` (struct :`R` 1.0 :`A` 1.0) :`true` (struct :`R` 1.0 :`G` 1.0 :`B` 1.0 :`A` 1.0) :!type "LinearColor Structure") null)
  (bind _isunitdead (`/Game/Match3RPGTemplate/Blueprints/Units/BP_UnitBase.IsUnitDead` (`self.player`)))
  (if _isunitdead
    (`self.KillPlayer`)
    (else
      (`/Game/Match3RPGTemplate/Blueprints/Units/BP_UnitBase.PlayAnimation` (`self.player`) (select `bool` _returnvalue :`false` "NewEnumerator4" :`true` "NewEnumerator0" :!type "/Game/Match3RPGTemplate/Blueprints/Units/AnimationType Enum")))))

(event `UsePlayerSkill`
  (params (playerSkill :type "/Game/Match3RPGTemplate/Blueprints/Skills/PlayerSkills/BP_PlayerSkillBase Object Reference"))
  ;[1 1 1] Player uses skill
  (if (== (`/Game/Match3RPGTemplate/Blueprints/Skills/BP_SkillBase.currentCooldown` playerSkill) 0)
    (if (<= (`/Game/Match3RPGTemplate/Blueprints/Skills/PlayerSkills/BP_PlayerSkillBase.manaCost` playerSkill) (`/Game/Match3RPGTemplate/Blueprints/Units/Player/BP_PlayerBase.currentMana` (`self.player`)))
      (`self.OnPlayerSkillActivated`)
      (`/Game/Match3RPGTemplate/Blueprints/Units/Player/BP_PlayerBase.ReduceMana` (`self.player`) (`/Game/Match3RPGTemplate/Blueprints/Skills/PlayerSkills/BP_PlayerSkillBase.manaCost` playerSkill))
      (`/Game/Match3RPGTemplate/Blueprints/Skills/PlayerSkills/BP_PlayerSkillBase.ResetCooldown` playerSkill)
      (`/Game/Match3RPGTemplate/Blueprints/Skills/BP_SkillBase.UseSkill` playerSkill)
      (else
        (bind _returnvalue (`|CreateWidget` "/Game/Match3RPGTemplate/Blueprints/UI/BP_InfoUI.BP_InfoUI_C" null true "Not Enough Mana!"))
        (`UserWidget.AddToViewport` _returnvalue 0)))))

(event `KillEnemy`
  ;[1 1 1] Enemy dies
  (bind _animationlength (`/Game/Match3RPGTemplate/Blueprints/Units/BP_UnitBase.PlayAnimation` (`self.currentEnemy`) "NewEnumerator5"))
  (`KismetSystemLibrary.Delay` _animationlength)
  (`/Game/Match3RPGTemplate/Blueprints/Units/BP_UnitBase.Dissolve` (`self.currentEnemy`))
  (`self.OnEnemyDied`)
  (`KismetArrayLibrary.Array_Clear` (`self.EnemySkills`))
  (set `self.enemyDieAnimationEnded` true)
  (if (`self.shouldSpawnNextEnemy`)
    (`self.SpawnNextEnemy`)))

(event `SpawnNextEnemy`
  ;[1 1 1] Spawns next enemy
  (`self.OnTurnEnded`)
  (bind _result (`/Engine/EditorBlueprintResources/StandardMacros.IncrementInt` (`self.currentEnemyIndex`))
    (:`  `
      (if (< _result (`KismetArrayLibrary.Array_Length` (`self.enemyList`)))
        (set `self.shouldSpawnNextEnemy` false)
        (set `self.enemyDieAnimationEnded` false)
        (`self.SpawnEnemy`)
        (else
          (`/Game/Match3RPGTemplate/Blueprints/Units/BP_UnitBase.PlayAnimation` (`self.player`) "NewEnumerator6")
          (`KismetSystemLibrary.Delay` 3.0)
          (`self.ResetAll`)
          (`self.OnAllEnemiesDied`))))))

(event `OnEnemyTurn`
  (bind _output (`|GetArrayItem` (`self.EnemySkills`)))
  ;[1 1 1] Enemy plays
  (bind _isunitdead (`/Game/Match3RPGTemplate/Blueprints/Units/BP_UnitBase.IsUnitDead` (`self.currentEnemy`)))
  (if _isunitdead
    (set `self.shouldSpawnNextEnemy` true)
    (if (`self.enemyDieAnimationEnded`)
      (`self.SpawnNextEnemy`))
    (else
      (bind _enemyskillcooldown (`self.GetEnemySkillCooldown`))
      (if (== _enemyskillcooldown 1)
        (add `/Game/Match3RPGTemplate/Blueprints/Skills/BP_SkillBase.OnSkillUsed` _output (delegate `OnEnemySkillUsedHandler`))
        (`/Game/Match3RPGTemplate/Blueprints/Skills/BP_SkillBase.UseSkill` _output)
        (else
          (`self.OnEnemyTurnEnded` :!label _label))))))

(event `OnEnemySkillUsedHandler`
  ;[1 1 1] Enemy plays
  (`self.RemoveUsedEnemySkillFromTheList`)
  (`self.OnEnemySkillUsed`)
  (goto _label))

(event `KillPlayer`
  ;[1 1 1] Player dies
  (bind _animationlength (`/Game/Match3RPGTemplate/Blueprints/Units/BP_UnitBase.PlayAnimation` (`self.player`) "NewEnumerator5"))
  (`KismetSystemLibrary.Delay` (+ _animationlength 2.0))
  (`/Game/Match3RPGTemplate/Blueprints/Units/BP_UnitBase.Dissolve` (`self.player`))
  (`KismetArrayLibrary.Array_Clear` (`self.EnemySkills`))
  (`self.ResetAll`)
  (`self.OnPlayerDied`))

(event `OnTurnEnded`
  ;[1 1 1] On turn ended
  (`self.ReduceEnemySkillCooldown`)
  (`self.ReducePlayerSkillCooldown`)
  (set `self.matchedShieldGemAmount` 0))

(event `ReduceEnemySkillCooldown`
  (bind _output (`|GetArrayItem` (`self.EnemySkills`)))
  ;[1 1 1] Reduce enemy skill cooldown
  (if (`self.wasEnemySkillUsed`)
    (set `self.wasEnemySkillUsed` false)
    (else
      (`/Engine/EditorBlueprintResources/StandardMacros.IsValid` _output
        (:`Is Valid`
          (`/Engine/EditorBlueprintResources/StandardMacros.DecrementInt` (`/Game/Match3RPGTemplate/Blueprints/Skills/BP_SkillBase.currentCooldown` _output)
            (:`  `
              (`self.OnEnemySkillCooldownUpdated`))))))))

(event `ReducePlayerSkillCooldown`
  ;[1 1 1] Reduce player skill cooldown
  (for _array_element (`self.playerSkills`)
    (`/Game/Match3RPGTemplate/Blueprints/Skills/PlayerSkills/BP_PlayerSkillBase.ReduceCooldown` _array_element)))

(event `RemoveUsedEnemySkillFromTheList`
  ;[1 1 1] Removes used enemy skill
  (`self.K2_DestroyActor` (`|GetArrayItem` (`self.EnemySkills`)))
  (`KismetArrayLibrary.Array_Remove` (`self.EnemySkills`))
  (`self.CreateEnemySkill` 1)
  (set `self.wasEnemySkillUsed` true))

(event `ResetAll`
  ;[1 1 1] Destroys actors
  (`self.K2_DestroyActor` (`self.stage`))
  (`|ExecutionSequence`
    (:`then_0`
      (`/Engine/EditorBlueprintResources/StandardMacros.IsValid` (`self.player`)
        (:`Is Valid`
          (`self.K2_DestroyActor` (`self.player`)))))
    (:`then_1`
      (`/Engine/EditorBlueprintResources/StandardMacros.IsValid` (`self.currentEnemy`)
        (:`Is Valid`
          (`self.K2_DestroyActor` (`self.currentEnemy`)))))))

(fn `GetCurrentEnemyAttackPower`
  (returns (enemyAttackPower :type Integer))
  (bind _output (`|GetArrayItem` (`self.EnemySkills`)))
  (`/Engine/EditorBlueprintResources/StandardMacros.IsValid` _output
    (:`Is Valid`
      (return (select `bool` (== (`/Game/Match3RPGTemplate/Blueprints/Skills/BP_SkillBase.currentCooldown` _output) 1) :`true` (`/Game/Match3RPGTemplate/Blueprints/Skills/BP_SkillBase.attackPower` _output))))
    (:`Is Not Valid`
      (return 0))))

(fn `GetEnemyDamage`
  (params (matchedDefenseGemAmount :type Integer))
  (returns (enemyDamage :type Integer))
  (bind _enemyattackpower (`self.GetCurrentEnemyAttackPower`))
  (bind _returnvalue (- _enemyattackpower (+ (* matchedDefenseGemAmount (`.DefenseMultiplier_7_3A9AAA3946899AD7CFC0D5892A33F0E9` (break `/Game/Match3RPGTemplate/Blueprints/Equipments/ShieldData` (`/Game/Match3RPGTemplate/Blueprints/BP_Match3RPGPlayerController.currentShield` (`self.match3RPGPlayerController`))))) (`/Game/Match3RPGTemplate/Blueprints/Units/BP_UnitBase.defense` (`self.player`)))))
  (return (`KismetMathLibrary.Clamp` _returnvalue 0 _returnvalue)))

(fn `GetEnemySkillBasedOnWeight`
  (returns (enemySkill :type "/Game/Match3RPGTemplate/Blueprints/Skills/EnemySkills/BP_EnemySkillBase Class Reference"))
  (locals (totalWeight :type "Float (double-precision)") (randomWeight :type "Float (double-precision)") (currentWeight :type "Float (double-precision)") (currentSkill :type "/Game/Match3RPGTemplate/Blueprints/Skills/EnemySkills/BP_EnemySkillBase Class Reference"))
  (bind _skills (`/Game/Match3RPGTemplate/Blueprints/Units/Enemy/BP_EnemyBase.skills` (`self.currentEnemy`)))
  (bind _values (`BlueprintMapLibrary.Map_Values` (`/Game/Match3RPGTemplate/Blueprints/Units/Enemy/BP_EnemyBase.skills` (`self.currentEnemy`))))
  (for _array_element _values
    (set `local.totalWeight` (+ _array_element (`local.totalWeight`))))
  (set `local.randomWeight` (`KismetMathLibrary.RandomFloatInRange` 0.0 (`local.totalWeight`)))
  (bind _keys (`BlueprintMapLibrary.Map_Keys` _skills))
  (for _array_element_2 _keys
    (set `local.currentWeight` (+ (`BlueprintMapLibrary.Map_Find` _skills _array_element_2) (`local.currentWeight`)))
    (if (<= (`local.randomWeight`) (`local.currentWeight`))
      (set `local.currentSkill` _array_element_2)
      (break)))
  (return (`local.currentSkill`)))

(fn `GetEnemySkillCooldown`
  (returns (enemySkillCooldown :type Integer))
  (bind _output (`|GetArrayItem` (`self.EnemySkills`)))
  (`/Engine/EditorBlueprintResources/StandardMacros.IsValid` _output
    (:`Is Valid`
      (return (`/Game/Match3RPGTemplate/Blueprints/Skills/BP_SkillBase.currentCooldown` _output)))
    (:`Is Not Valid`
      (return 0))))

(fn `GetGems`
  (returns (gems :type "Array of /Game/Match3RPGTemplate/Blueprints/Gems/BP_GemBase Class Reference"))
  (locals (allGems :type "Array of /Game/Match3RPGTemplate/Blueprints/Gems/BP_GemBase Class Reference"))
  (`KismetArrayLibrary.Array_Append` (`local.allGems`) (`/Game/Match3RPGTemplate/Blueprints/Units/Player/BP_PlayerBase.characterGems` (`self.player`)))
  (`KismetArrayLibrary.Array_Append` (`local.allGems`) (`.Gems_13_B30762F34746D73708F65A9A53DAEC97` (break `/Game/Match3RPGTemplate/Blueprints/Equipments/ArmorData` (`/Game/Match3RPGTemplate/Blueprints/BP_Match3RPGPlayerController.currentArmor` (`self.match3RPGPlayerController`)))))
  (`KismetArrayLibrary.Array_Append` (`local.allGems`) (`.Gems_16_6BA6CA67448877E1D728A38E93E61CC3` (break `/Game/Match3RPGTemplate/Blueprints/Equipments/WeaponData` (`/Game/Match3RPGTemplate/Blueprints/BP_Match3RPGPlayerController.currentWeapon` (`self.match3RPGPlayerController`)))))
  (`KismetArrayLibrary.Array_Append` (`local.allGems`) (`.Gems_15_77CC0C6C4F55991C54410F880B7915B4` (break `/Game/Match3RPGTemplate/Blueprints/Equipments/ShieldData` (`/Game/Match3RPGTemplate/Blueprints/BP_Match3RPGPlayerController.currentShield` (`self.match3RPGPlayerController`)))))
  (return (`local.allGems`)))

(fn `GetPlayerDamage`
  (params (matchedAttackGemAmount :type Integer))
  (returns (playerDamage :type Integer))
  (bind _returnvalue (- (+ (* matchedAttackGemAmount (`.AttackMultiplier_8_2FCFF42648C9978966732CB718FA7B83` (break `/Game/Match3RPGTemplate/Blueprints/Equipments/WeaponData` (`/Game/Match3RPGTemplate/Blueprints/BP_Match3RPGPlayerController.currentWeapon` (`self.match3RPGPlayerController`))))) (`/Game/Match3RPGTemplate/Blueprints/Units/Player/BP_PlayerBase.attackPower` (`self.player`))) (`/Game/Match3RPGTemplate/Blueprints/Units/BP_UnitBase.defense` (`self.currentEnemy`))))
  (return (`KismetMathLibrary.Clamp` _returnvalue 0 _returnvalue)))

(fn `GetPlayerSkills`
  (returns (playerSkills :type "Array of /Game/Match3RPGTemplate/Blueprints/Skills/PlayerSkills/BP_PlayerSkillBase Class Reference"))
  (locals (allSkills :type "Array of /Game/Match3RPGTemplate/Blueprints/Skills/PlayerSkills/BP_PlayerSkillBase Class Reference"))
  (`KismetArrayLibrary.Array_Append` (`local.allSkills`) (`/Game/Match3RPGTemplate/Blueprints/Units/Player/BP_PlayerBase.skills` (`self.player`)))
  (`KismetArrayLibrary.Array_Append` (`local.allSkills`) (`.Skills_15_C93D02AF443FEC8134981DB1AB28D6CD` (break `/Game/Match3RPGTemplate/Blueprints/Equipments/ArmorData` (`/Game/Match3RPGTemplate/Blueprints/BP_Match3RPGPlayerController.currentArmor` (`self.match3RPGPlayerController`)))))
  (`KismetArrayLibrary.Array_Append` (`local.allSkills`) (`.Skills_13_F6EB0752464D66883570DB96F770359C` (break `/Game/Match3RPGTemplate/Blueprints/Equipments/WeaponData` (`/Game/Match3RPGTemplate/Blueprints/BP_Match3RPGPlayerController.currentWeapon` (`self.match3RPGPlayerController`)))))
  (`KismetArrayLibrary.Array_Append` (`local.allSkills`) (`.Skills_12_C763533B4F05AA55546274A595F15893` (break `/Game/Match3RPGTemplate/Blueprints/Equipments/ShieldData` (`/Game/Match3RPGTemplate/Blueprints/BP_Match3RPGPlayerController.currentShield` (`self.match3RPGPlayerController`)))))
  (return (`local.allSkills`)))

(fn `UserConstructionScript`)