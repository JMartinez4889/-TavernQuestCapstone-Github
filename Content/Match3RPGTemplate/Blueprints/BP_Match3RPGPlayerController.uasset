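; Player controller for a match-3 RPG that handles gem-linking input, creates the game UI and tracks gold and owned or equipped gear.
; Gem drags chain adjacent identical gems with backtracking, gated by matching turn and board state.
; Releasing three or more fires match completion with the unbroken-gem count, which also feeds a details popup following the mouse, or the current slot on mobile.
; Skills route to the BattleManager; equipment resolves from Shop data tables.
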(event `SetupPlayer`
  (params (shop :type "/Game/Match3RPGTemplate/Blueprints/BP_Shop Object Reference") (player :type "/Game/Match3RPGTemplate/Blueprints/Units/Player/BP_PlayerBase Class Reference"))
  (bind (_overhealth _startingitems _startinggold) (defaults `Object` player))
  (bind (_startingarmor _startingweapon _startingshield) (break `/Game/Match3RPGTemplate/Blueprints/StartingItems` _startingitems))
  (bind (_datatable _rowname) (break `DataTableRowHandle` _startingweapon))
  (bind (_datatable_2 _rowname_2) (break `DataTableRowHandle` _startingarmor))
  (bind (_datatable_3 _rowname_3) (break `DataTableRowHandle` _startingshield))
  ;[1 1 1] Setup player
  (set `self.shop` shop)
  (`self.OnArmorOwned` _rowname_2)
  (`self.SetCurrentArmor` _rowname_2)
  (`self.OnWeaponOwned` _rowname)
  (`self.SetCurrentWeapon` _rowname)
  (`self.OnShieldOwned` _rowname_3)
  (`self.SetCurrentShield` _rowname_3)
  (set `self.currentGold` _startinggold))

(event `CreateGameUI`
  (params (battleManager :type "/Game/Match3RPGTemplate/Blueprints/BP_BattleManager Object Reference") (gemList :type "Array of /Game/Match3RPGTemplate/Blueprints/Gems/BP_GemBase Object Reference") (match3RPGController :type "/Game/Match3RPGTemplate/Blueprints/BP_Match3RPGController Object Reference"))
  ;[1 1 1] Create game UI
  (set `self.battleManager` battleManager)
  (add `/Game/Match3RPGTemplate/Blueprints/BP_Match3RPGController.OnGameStateChanged` match3RPGController (delegate `OnGameStateChangedHandler`))
  (bind _returnvalue (`|CreateWidget` "/Game/Match3RPGTemplate/Blueprints/UI/BP_GameUI.BP_GameUI_C" null gemList self))
  (bind _output_get (set `self.GameUI` _returnvalue))
  (`/Game/Match3RPGTemplate/Blueprints/UI/BP_GameUI.SetPlayerInfo` _output_get (`self.battleManager`))
  (`/Game/Match3RPGTemplate/Blueprints/UI/BP_GameUI.UpdateGoldAmount` (`self.GameUI`) (`self.currentGold`))
  (`UserWidget.AddToViewport` (`self.GameUI`) 0)
  (`WidgetBlueprintLibrary.SetInputMode_UIOnlyEx` self null)
  (add `/Game/Match3RPGTemplate/Blueprints/BP_BattleManager.OnEnemySpawned` (`self.battleManager`) (delegate `OnEnemySpawnedhandler`))
  (bind _returnvalue_2 (`|CreateWidget` "/Game/Match3RPGTemplate/Blueprints/UI/BP_MatchingDetailsUI.BP_MatchingDetailsUI_C"))
  (bind _output_get_2 (set `self.matchingDetailsUI` _returnvalue_2))
  (`UserWidget.AddToViewport` _output_get_2 0)
  (`self.HidematchingDetailsUI`))

(event `OnEnemySpawnedhandler`
  ;[1 1 1] Create game UI
  (`/Game/Match3RPGTemplate/Blueprints/UI/BP_GameUI.SetEnemyInfo` (`self.GameUI`) (`self.battleManager`)))

(event `OnGameStateChangedHandler`
  (params (gameState :type "/Game/Match3RPGTemplate/Blueprints/GameState Enum" :default "NewEnumerator1"))
  ;[1 1 1] Create game UI
  (`self.RemoveUI` gameState)
  (if (`|EnumEquality` gameState "NewEnumerator2")
    (set `self.isMatchingTurn` true)
    (`/Game/Match3RPGTemplate/Blueprints/UI/BP_GameUI.ShowCountdown` (`self.GameUI`) (`self.battleManager`))
    (else
      (set `self.isMatchingTurn` false))))

(event `RemoveUI`
  (params (gameState :type "/Game/Match3RPGTemplate/Blueprints/GameState Enum" :default "NewEnumerator1"))
  ;[1 1 1] Create game UI
  (if (`|EnumEquality` gameState "NewEnumerator6")
    (`Widget.RemoveFromParent` (`self.GameUI`))))

(event `OnGemDragStarted`
  (params (gem :type "/Game/Match3RPGTemplate/Blueprints/Gems/BP_GemBase Object Reference") (slot :type "/Game/Match3RPGTemplate/Blueprints/UI/BP_Slot Object Reference"))
  ;[1 1 1] Start dragging gem
  (`self.CanPlayerPlay`
    (:`CanPlay`
      (`/Engine/EditorBlueprintResources/StandardMacros.IsValid` (`self.draggingGem`)
        (:`Is Not Valid`
          (set `self.draggingGem` gem)
          (bind _output_get (set `self.currentSlot` slot))
          (`/Game/Match3RPGTemplate/Blueprints/UI/BP_Slot.SetSlotSelected` _output_get)
          (`/Game/Match3RPGTemplate/Blueprints/UI/BP_GameUI.BlockNonMatchingGems` (`self.GameUI`) (`self.draggingGem`))
          (`KismetArrayLibrary.Array_Add` (`self.matchedGemSlots`) (`self.currentSlot`))
          (`self.UpdateMatchingDetails`)
          (`self.ShowMatchingDetailsUI`))))))

(event `OnGemDragged`
  (params (gem :type "/Game/Match3RPGTemplate/Blueprints/Gems/BP_GemBase Object Reference") (slot :type "/Game/Match3RPGTemplate/Blueprints/UI/BP_Slot Object Reference"))
  ;[1 1 1] Gem is being dragged
  (`self.CanPlayerPlay`
    (:`CanPlay`
      (if (`KismetArrayLibrary.Array_Contains` (`self.matchedGemSlots`) slot)
        (`self.ReAdjustTheLink` slot)
        (`self.UpdateMatchingDetails`)
        (else
          (bind (_areslotsadjacent _angle _isdiagonal) (`/Game/Match3RPGTemplate/Blueprints/UI/BP_GameUI.AreSlotsAdjacent` (`self.GameUI`) (`self.currentSlot`) slot))
          (if (and _areslotsadjacent (== gem (`self.draggingGem`)))
            (`/Game/Match3RPGTemplate/Blueprints/UI/BP_Slot.SetSlotSelected` slot)
            (`KismetArrayLibrary.Array_Add` (`self.matchedGemSlots`) slot)
            (`/Game/Match3RPGTemplate/Blueprints/UI/BP_Slot.ShowLink` (`self.currentSlot`) _angle _isdiagonal)
            (set `self.currentSlot` slot)
            (`self.UpdateMatchingDetails`)))))))

(event `OnGemDragEnded`
  ;[1 1 1] Gem drag ended
  (`self.CanPlayerPlay`
    (:`CanPlay`
      (`self.HidematchingDetailsUI`)
      (if (>= (`KismetArrayLibrary.Array_Length` (`self.matchedGemSlots`)) 3)
        (`self.MatchingCompleted`))
      (set `self.draggingGem` null)
      (set `self.currentSlot` null)
      (`/Game/Match3RPGTemplate/Blueprints/UI/BP_GameUI.ResetSlotEffects` (`self.GameUI`))
      (`KismetArrayLibrary.Array_Clear` (`self.matchedGemSlots`)))))

(event `MatchingCompleted`
  (bind _matchedgemslots (`self.matchedGemSlots`))
  ;[1 1 1] On gem match completed
  (`/Game/Match3RPGTemplate/Blueprints/UI/BP_GameUI.MatchingCompleted` (`self.GameUI`) _matchedgemslots)
  (bind _nonbrokengemslots (`self.GetNonBrokenMatchedGems` _matchedgemslots))
  (`self.OnMatchCompleted` (`self.draggingGem`) _nonbrokengemslots))

(event `UpdateMatchingDetails`
  ;[1 1 1] Update matching details
  (bind _nonbrokengemslots (`self.GetNonBrokenMatchedGems` (`self.matchedGemSlots`)))
  (`/Game/Match3RPGTemplate/Blueprints/Gems/BP_GemBase.UpdateMatchingDetails` (`self.draggingGem`) (`self.matchingDetailsUI`) _nonbrokengemslots))

(event `ShowMatchingDetailsUI`
  ;[1 1 1] Enable / Disable matching details UI
  (`Widget.SetVisibility` (`self.matchingDetailsUI`) "HitTestInvisible"))

(event `HideMatchingDetailsUI`
  ;[1 1 1] Enable / Disable matching details UI
  (`Widget.SetVisibility` (`self.matchingDetailsUI`) "Hidden"))

(event `self.ReceiveTick`
  (params (DeltaSeconds :type "Float (single-precision)"))
  (bind _returnvalue (`Widget.GetCachedGeometry` (`self.currentSlot`)))
  ;[1 1 1] Set matching details UI position
  (`/Engine/EditorBlueprintResources/StandardMacros.IsValid` (`self.matchingDetailsUI`)
    (:`Is Valid`
      (`/Engine/EditorBlueprintResources/StandardMacros.IsValid` (`self.currentSlot`)
        (:`Is Valid`
          (switch `string` (`GameplayStatics.GetPlatformName`)
            (:`Default`
              (bind _returnvalue_2 (`WidgetLayoutLibrary.GetMousePositionOnViewport`))
              (`UserWidget.SetPositionInViewport` (`self.matchingDetailsUI`) _returnvalue_2 false))
            (:`Android`
              (`UserWidget.SetPositionInViewport` (`self.matchingDetailsUI`) (+ (* (`SlateBlueprintLibrary.GetLocalSize` _returnvalue) 0.5) (`.ViewportPosition` (`SlateBlueprintLibrary.LocalToViewport` _returnvalue))) false :!label _label))
            (:`IOS`
              (goto _label))))))))

(event `UseSkill`
  (params (playerSkill :type "/Game/Match3RPGTemplate/Blueprints/Skills/PlayerSkills/BP_PlayerSkillBase Object Reference"))
  ;[1 1 1] Use Skill
  (`self.CanPlayerPlay`
    (:`CanPlay`
      (`/Game/Match3RPGTemplate/Blueprints/BP_BattleManager.UsePlayerSkill` (`self.battleManager`) playerSkill))))

(event `IncreaseGold`
  (params (goldAmount :type Integer))
  ;[1 1 1] Increase gold
  (bind _output_get (set `self.currentGold` (+ goldAmount (`self.currentGold`))))
  (`/Game/Match3RPGTemplate/Blueprints/UI/BP_GameUI.UpdateGoldAmount` (`self.GameUI`) _output_get))

(event `SpendGold`
  (params (goldAmount :type Integer))
  (bind _returnvalue (- (`self.currentGold`) goldAmount))
  ;[1 1 1] Decrease gold
  (set `self.currentGold` (`KismetMathLibrary.Clamp` _returnvalue 0 _returnvalue)))

(event `SetCurrentWeapon`
  (params (weaponID :type Name))
  ;[1 1 1] Equip / set gears
  (bind _output_get (set `self.currentWeaponID` weaponID))
  (bind _returnvalue (`|GetDataTableRow` (`/Game/Match3RPGTemplate/Blueprints/BP_Shop.WeaponShop` (`self.shop`)) _output_get)
    (:`then`
      (set `self.currentWeapon` _returnvalue))))

(event `SetCurrentArmor`
  (params (armorID :type Name))
  ;[1 1 1] Equip / set gears
  (bind _output_get (set `self.currentArmorID` armorID))
  (bind _returnvalue (`|GetDataTableRow` (`/Game/Match3RPGTemplate/Blueprints/BP_Shop.ArmorShop` (`self.shop`)) _output_get)
    (:`then`
      (set `self.currentArmor` _returnvalue))))

(event `SetCurrentShield`
  (params (shieldID :type Name))
  ;[1 1 1] Equip / set gears
  (bind _output_get (set `self.currentShieldID` shieldID))
  (bind _returnvalue (`|GetDataTableRow` (`/Game/Match3RPGTemplate/Blueprints/BP_Shop.ShieldShop` (`self.shop`)) _output_get)
    (:`then`
      (set `self.currentShield` _returnvalue))))

(event `OnWeaponOwned`
  (params (weaponID :type Name))
  ;[1 1 1] Equip / set gears
  (`KismetArrayLibrary.Array_AddUnique` (`self.ownedWeapons`) weaponID))

(event `OnArmorOwned`
  (params (armorID :type Name))
  ;[1 1 1] Equip / set gears
  (`KismetArrayLibrary.Array_AddUnique` (`self.ownedArmors`) armorID))

(event `OnShieldOwned`
  (params (shieldID :type Name))
  ;[1 1 1] Equip / set gears
  (`KismetArrayLibrary.Array_AddUnique` (`self.ownedShields`) shieldID))

(event `OnCharacterOwned`
  (params (CharacterID :type String))
  ;[1 1 1] Equip / set gears
  (`KismetArrayLibrary.Array_AddUnique` (`self.ownedCharacters`) (`KismetStringLibrary.Conv_StringToName` CharacterID)))

(fn `GetNonBrokenMatchedGems`
  (params (matchedGemSlots :type "Array of /Game/Match3RPGTemplate/Blueprints/UI/BP_Slot Object Reference"))
  (returns (nonBrokenGemSlots :type Integer))
  (locals (nonBrokenGemSlotCount :type Integer :default 0))
  (for _array_element matchedGemSlots
    (if (not (`/Game/Match3RPGTemplate/Blueprints/UI/BP_Slot.isBroken` _array_element))
      (`/Engine/EditorBlueprintResources/StandardMacros.IncrementInt` (`local.nonBrokenGemSlotCount`))))
  (return (`local.nonBrokenGemSlotCount`)))

(fn `ReAdjustTheLink`
  (params (slot :type "/Game/Match3RPGTemplate/Blueprints/UI/BP_Slot Object Reference"))
  (returns (adjusted :type Boolean))
  (bind (_arrayindex _arrayelement) (`/Engine/EditorBlueprintResources/StandardMacros.ReverseForEachLoop` (`self.matchedGemSlots`))
    (:`LoopBody`
      (if (!= _arrayelement slot)
        (`/Game/Match3RPGTemplate/Blueprints/UI/BP_Slot.ResetSlotEffect` _arrayelement)
        (`KismetArrayLibrary.Array_RemoveItem` (`self.matchedGemSlots`) _arrayelement)
        (else
          (`/Game/Match3RPGTemplate/Blueprints/UI/BP_Slot.ResetSlotEffect` _arrayelement)
          (`/Game/Match3RPGTemplate/Blueprints/UI/BP_Slot.SetSlotSelected` _arrayelement)
          (set `self.currentSlot` _arrayelement)
          (return true))))
    (:`Completed`
      (return false))))

(fn `UserConstructionScript`)