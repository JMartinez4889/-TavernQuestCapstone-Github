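; BP_Obliterate is a Witch player skill that performs an attack on the enemy in the Match-3 RPG.
; UseSkill moves the player to the enemy, then plays an attack animation and applies AttackPower damage through BattleManager at the animation's hit delay.
; After the remaining animation time, the player moves back and the skill signals completion through CallOnSkillUsed.
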(event `self.UseSkill`
  ;[1 1 1] Move player next to enemy
  (`self.PlayerMove` (delegate `OnMovedToEnemyHandler`)))

(event `OnMovedToEnemyHandler`
  ;[1 1 1] Move player next to enemy
  (`self.PlayAttack`))

(event `PlayAttack`
  (bind _player (`/Game/Match3RPGTemplate/Blueprints/BP_BattleManager.player` (`self.battleManager`)))
  (bind _animationhitdelay (`/Game/Match3RPGTemplate/Blueprints/Units/BP_UnitBase.animationHitDelay` _player))
  ;[1 1 1] Player unit attacks
  (bind _animationlength (`/Game/Match3RPGTemplate/Blueprints/Units/BP_UnitBase.PlayAnimation` _player "NewEnumerator3"))
  (`KismetSystemLibrary.Delay` _animationhitdelay)
  (`/Game/Match3RPGTemplate/Blueprints/BP_BattleManager.PlayerDoDamage` (`self.battleManager`) (`self.attackPower`))
  (bind _returnvalue (- _animationlength _animationhitdelay))
  (`KismetSystemLibrary.Delay` (select `bool` (> _returnvalue 0.0) :`true` _returnvalue))
  (`self.PlayerMoveBack` (delegate `OnPlayerMovedBackHandler`)))

(event `OnPlayerMovedBackHandler`
  ;[1 1 1] Player unit attacks
  (`self.OnSkillUsed`))

(fn `UserConstructionScript`
  (`parent.UserConstructionScript`))