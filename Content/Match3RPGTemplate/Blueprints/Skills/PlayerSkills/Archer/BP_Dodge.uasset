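; Archer player skill for the match-3 RPG that guards against the current enemy attack.
; On use it reads the enemy's attack power from the BattleManager and, if nonzero, plays the player's guard animation and sets the matched shield gem amount to a fixed value.
; It fires OnSkillUsed in both cases, so use against a zero-power attack still completes without any defensive effect.
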(event `self.UseSkill`
  ;[1 1 1] Play guard animation
  (bind _enemyattackpower (`/Game/Match3RPGTemplate/Blueprints/BP_BattleManager.GetCurrentEnemyAttackPower` (`self.battleManager`)))
  (if (== _enemyattackpower 0)
    (`self.OnSkillUsed`)
    (else
      (`/Game/Match3RPGTemplate/Blueprints/Units/BP_UnitBase.PlayAnimation` (`/Game/Match3RPGTemplate/Blueprints/BP_BattleManager.player` (`self.battleManager`)) "NewEnumerator7")
      (set `/Game/Match3RPGTemplate/Blueprints/BP_BattleManager.matchedShieldGemAmount` 10 (`self.battleManager`))
      (`self.OnSkillUsed`))))

(fn `UserConstructionScript`
  (`parent.UserConstructionScript`))