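; Central game controller for a match-3 RPG, running the flow from main menu through turn-based stage battles to game over.
; A game-state switch spawns and initializes the battle manager, then cycles enemy spawn, player matching, enemy turn and end turn via event callbacks.
; It spawns gems from the battle manager and routes completed matches to their effects.
; Character selection swaps the active player and equips its data-table weapon, armor and shield.
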(event `Change`
  (params (SelectedCharacter :type Name))
  (bind _match3rpgplayercontroller (`self.match3RPGPlayerController`))
  (bind _invuiref (`self.CharacterSwap` SelectedCharacter))
  (bind _returnvalue (`|GetDataTableRow` "/Game/Match3RPGTemplate/Blueprints/CharacterDataTable.CharacterDataTable" SelectedCharacter)
    (:`then`
      (bind ((`WeaponID_44_67A74CA745C6E57EEC943FB2D5D1D52C` _weaponid) (`ArmorID_45_08061768409E46C291F661B165C7A3E3` _armorid) (`ShieldID_46_49035C864F57BBA0A43BE88767701211` _shieldid)) (break `/Game/Match3RPGTemplate/Blueprints/CharactersStruct` _returnvalue))
      (`/Game/Match3RPGTemplate/Blueprints/BP_Match3RPGPlayerController.SetCurrentWeapon` _match3rpgplayercontroller _weaponid)
      (`/Game/Match3RPGTemplate/Blueprints/BP_Match3RPGPlayerController.SetCurrentArmor` _match3rpgplayercontroller _armorid)
      (`/Game/Match3RPGTemplate/Blueprints/BP_Match3RPGPlayerController.SetCurrentShield` _match3rpgplayercontroller _shieldid)
      (`/Game/Match3RPGTemplate/Blueprints/UI/Equipments/BP_InventoryUI.ShowAllStats` _invuiref))))

(event `self.ReceiveBeginPlay`
  ;[1 1 1] Setup player
  (bind _asbp_match_3rpgplayer_controller (cast `/Game/Match3RPGTemplate/Blueprints/BP_Match3RPGPlayerController` (`GameplayStatics.GetPlayerController` 0))
    (:`then`
      (bind _output_get (set `self.match3RPGPlayerController` _asbp_match_3rpgplayer_controller))
      (bind _outactors (`GameplayStatics.GetAllActorsOfClass` "/Game/Match3RPGTemplate/Blueprints/BP_MainMenuController.BP_MainMenuController_C"))
      (set `self.MainMenuUIRef` (`|GetArrayItem` _outactors))
      (`/Game/Match3RPGTemplate/Blueprints/BP_Match3RPGPlayerController.SetupPlayer` _output_get (`self.shop`) (`self.player`))
      (`self.ShowMainMenu`))
    (:`CastFailed`
      (`KismetSystemLibrary.PrintString` "Match3RPGPlayerController is NOT assigned GameMode" true true (struct :`R` 1.0 :`A` 1.0) 5.0))))

(event `ShowMainMenu`
  (bind _mainmenucontroller (`self.mainMenuController`))
  ;[1 1 1] Show main menu
  (`/Game/Match3RPGTemplate/Blueprints/BP_MainMenuController.ShowMainMenu` _mainmenucontroller (`self.player`) (`self.shop`))
  (add `/Game/Match3RPGTemplate/Blueprints/BP_MainMenuController.OnStageSelected` _mainmenucontroller (delegate `OnStageSelectedhandler`)))

(event `OnStageSelectedhandler`
  (params (stageData :type "/Game/Match3RPGTemplate/Blueprints/StageData Structure"))
  ;[1 1 1] Show main menu
  (set `self.stageData` stageData)
  (set `self.playerWon` false)
  (`self.ChangeGameState` "NewEnumerator1"))

(event `ChangeGameState`
  (params (gameState :type "/Game/Match3RPGTemplate/Blueprints/GameState Enum" :default "NewEnumerator1"))
  ;[1 1 1] Change game state
  (bind _output_get (set `self.gameState` gameState))
  (`self.OnGameStateChanged` _output_get)
  (switch `/Game/Match3RPGTemplate/Blueprints/GameState` (`self.gameState`)
    (:`NewEnumerator1`
      (`self.Initialization`))
    (:`NewEnumerator7`
      (`self.SpawnEnemy`))
    (:`NewEnumerator4`
      (`self.EnemiesTurn`))
    (:`NewEnumerator5`
      (`self.EndTurn`))
    (:`NewEnumerator6`
      (`self.GameOver`))))

(event `Initialization`
  ;[1 1 1] UInitialize and set all the callbacks
  (bind _returnvalue (`|SpawnActorFromClass` "/Game/Match3RPGTemplate/Blueprints/BP_BattleManager.BP_BattleManager_C" (`KismetMathLibrary.MakeTransform` (0.0 0.0 0.0)) "Undefined" "OverrideRootScale" null null))
  (bind _output_get (set `self.battleManager` _returnvalue))
  (add `/Game/Match3RPGTemplate/Blueprints/BP_BattleManager.OnBattleManagerInitialized` _output_get (delegate `OnBattleManagerInitializedHandler`))
  (`/Game/Match3RPGTemplate/Blueprints/BP_BattleManager.Initialize` (`self.battleManager`) (`self.player`) (`self.stageData`))
  (add `/Game/Match3RPGTemplate/Blueprints/BP_BattleManager.OnEnemySpawned` (`self.battleManager`) (delegate `OnEnemySpawnedHandler`))
  (add `/Game/Match3RPGTemplate/Blueprints/BP_BattleManager.OnPlayerSkillActivated` (`self.battleManager`) (delegate `OnPlayerSkillActivatedHandler`))
  (add `/Game/Match3RPGTemplate/Blueprints/BP_BattleManager.OnPlayerSkillUsed` (`self.battleManager`) (delegate `OnPlayerSkillUsedHandler`))
  (add `/Game/Match3RPGTemplate/Blueprints/BP_BattleManager.OnEnemyTurnEnded` (`self.battleManager`) (delegate `OnEnemyTurnEndedHandler`))
  (add `/Game/Match3RPGTemplate/Blueprints/BP_BattleManager.OnAllEnemiesDied` (`self.battleManager`) (delegate `OnAllEnemiesDiedHandler`))
  (add `/Game/Match3RPGTemplate/Blueprints/BP_BattleManager.OnPlayerDied` (`self.battleManager`) (delegate `OnPlayerDiedHandler`)))

(event `OnPlayerSkillUsedHandler`
  ;[1 1 1] UInitialize and set all the callbacks
  (`self.ChangeGameState` "NewEnumerator4"))

(event `OnPlayerDiedHandler`
  ;[1 1 1] UInitialize and set all the callbacks
  (`self.ChangeGameState` "NewEnumerator6" :!label _label))

(event `OnAllEnemiesDiedHandler`
  ;[1 1 1] UInitialize and set all the callbacks
  (set `self.playerWon` true)
  (goto _label))

(event `OnPlayerSkillActivatedHandler`
  ;[1 1 1] UInitialize and set all the callbacks
  (`self.ChangeGameState` "NewEnumerator8"))

(event `OnEnemySpawnedHandler`
  ;[1 1 1] UInitialize and set all the callbacks
  (`KismetSystemLibrary.Delay` 0.5)
  (`self.ChangeGameState` "NewEnumerator2"))

(event `OnEnemyTurnEndedHandler`
  ;[1 1 1] UInitialize and set all the callbacks
  (`self.ChangeGameState` "NewEnumerator5"))

(event `OnBattleManagerInitializedHandler`
  ;[1 1 1] UInitialize and set all the callbacks
  (`self.CreateGems`)
  (`self.ChangeGameState` "NewEnumerator7"))

(event `CreateGems`
  ;[1 1 1] Spawn gems
  (`KismetArrayLibrary.Array_Clear` (`self.gemList`))
  (bind _gems (`/Game/Match3RPGTemplate/Blueprints/BP_BattleManager.GetGems` (`self.battleManager`)))
  (for _array_element _gems
    (bind _returnvalue (`|SpawnActorFromClass` _array_element (`KismetMathLibrary.MakeTransform` (0.0 0.0 0.0)) "Undefined" "OverrideRootScale" null (`self.battleManager`) (`self.match3RPGPlayerController`) null))
    (add `/Game/Match3RPGTemplate/Blueprints/Gems/BP_GemBase.OnPlayersTurnEnded` _returnvalue (delegate `OnPlayersTurnEndedHandler`))
    (`KismetArrayLibrary.Array_Add` (`self.gemList`) _returnvalue))
  (`self.CreateGameUI`))

(event `OnPlayersTurnEndedHandler`
  ;[1 1 1] Spawn gems
  (`self.ChangeGameState` "NewEnumerator4"))

(event `CreateGameUI`
  ;[1 1 1] Create game UI
  (`/Game/Match3RPGTemplate/Blueprints/BP_Match3RPGPlayerController.CreateGameUI` (`self.match3RPGPlayerController`) (`self.battleManager`) (`self.gemList`) self)
  (add `/Game/Match3RPGTemplate/Blueprints/BP_Match3RPGPlayerController.OnMatchCompleted` (`self.match3RPGPlayerController`) (delegate `OnMatchCompletedHandler`)))

(event `OnMatchCompletedHandler`
  (params (matchedGem :type "/Game/Match3RPGTemplate/Blueprints/Gems/BP_GemBase Object Reference") (matchedGemAmount :type Integer))
  ;[1 1 1] Create game UI
  (`self.ChangeGameState` "NewEnumerator8")
  (`/Game/Match3RPGTemplate/Blueprints/Gems/BP_GemBase.OnMatch` matchedGem matchedGemAmount))

(event `SpawnEnemy`
  ;[1 1 1] Spawn enemy
  (`/Game/Match3RPGTemplate/Blueprints/BP_BattleManager.SpawnEnemy` (`self.battleManager`)))

(event `EnemiesTurn`
  ;[1 1 1] Enemy plays
  (`KismetSystemLibrary.Delay` 0.5)
  (`/Game/Match3RPGTemplate/Blueprints/BP_BattleManager.OnEnemyTurn` (`self.battleManager`)))

(event `EndTurn`
  ;[1 1 1] On turn ended
  (`/Game/Match3RPGTemplate/Blueprints/BP_BattleManager.OnTurnEnded` (`self.battleManager`))
  (`KismetSystemLibrary.Delay` 0.5)
  (`self.ChangeGameState` "NewEnumerator2"))

(event `GameOver`
  ;[1 1 1] Game over
  (if (`self.playerWon`)
    (`/Game/Match3RPGTemplate/Blueprints/BP_MainMenuController.OnStageCleared` (`self.mainMenuController`))
    (`self.ShowMainMenu`)
    (else
      (bind _returnvalue (`|CreateWidget` "/Game/Match3RPGTemplate/Blueprints/UI/W_LSkinUI.W_LSkinUI_C"))
      (`UserWidget.AddToViewport` _returnvalue 0))))

(event `End`
  (`self.ShowMainMenu`))

(fn `CharacterSwap`
  (params (Selection :type Name))
  (returns (InvUIRef :type "/Game/Match3RPGTemplate/Blueprints/UI/Equipments/BP_InventoryUI Object Reference"))
  (bind _invuiref (`/Game/Match3RPGTemplate/Blueprints/UI/MainMenu/BP_MainMenu.InvUIRef` (`/Game/Match3RPGTemplate/Blueprints/BP_MainMenuController.mainMenu` (`self.mainMenuController`))))
  (switch `name` Selection
    (:`Warrior`
      (bind _output_get (set `self.player` "/Game/Match3RPGTemplate/Blueprints/Units/Player/Warrior.Warrior_C"))
      (set `/Game/Match3RPGTemplate/Blueprints/UI/Equipments/BP_InventoryUI.player` _output_get _invuiref))
    (:`Mage`
      (bind _output_get_2 (set `self.player` "/Game/Match3RPGTemplate/Blueprints/Units/Player/Mage.Mage_C"))
      (set `/Game/Match3RPGTemplate/Blueprints/UI/Equipments/BP_InventoryUI.player` _output_get_2 _invuiref))
    (:`Wizard`
      (bind _output_get_3 (set `self.player` "/Game/Match3RPGTemplate/Blueprints/Units/Player/Wizard.Wizard_C"))
      (set `/Game/Match3RPGTemplate/Blueprints/UI/Equipments/BP_InventoryUI.player` _output_get_3 _invuiref))
    (:`Witch`
      (bind _output_get_4 (set `self.player` "/Game/Match3RPGTemplate/Blueprints/Units/Player/Witch.Witch_C"))
      (set `/Game/Match3RPGTemplate/Blueprints/UI/Equipments/BP_InventoryUI.player` _output_get_4 _invuiref))
    (:`Archer`
      (bind _output_get_5 (set `self.player` "/Game/Match3RPGTemplate/Blueprints/Units/Player/Archer.Archer_C"))
      (set `/Game/Match3RPGTemplate/Blueprints/UI/Equipments/BP_InventoryUI.player` _output_get_5 _invuiref))
    (:`Knight`
      (bind _output_get_6 (set `self.player` "/Game/Match3RPGTemplate/Blueprints/Units/Player/Knight.Knight_C"))
      (set `/Game/Match3RPGTemplate/Blueprints/UI/Equipments/BP_InventoryUI.player` _output_get_6 _invuiref))
    (:`Pixie`
      (bind _output_get_7 (set `self.player` "/Game/Match3RPGTemplate/Blueprints/Units/Player/Pixie.Pixie_C"))
      (set `/Game/Match3RPGTemplate/Blueprints/UI/Equipments/BP_InventoryUI.player` _output_get_7 _invuiref)))
  (return _invuiref))

(fn `UserConstructionScript`)