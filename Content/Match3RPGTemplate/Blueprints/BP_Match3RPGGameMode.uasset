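; BP_Match3RPGGameMode is the game mode for the Match-3 RPG template and handles player respawning.
; PostLogin stores the joining player's controller and restarts it, and each restart binds the controlled pawn's OnDestroyed event to PlayerDied.
; PlayerDied restarts that stored player, so only the most recently logged-in player is tracked.
; BeginPlay also caches the first BP_Match3RPGController found, though this graph never uses it.
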(event `self.ReceiveBeginPlay`
  (bind _outactors (`GameplayStatics.GetAllActorsOfClass` "/Game/Match3RPGTemplate/Blueprints/BP_Match3RPGController.BP_Match3RPGController_C"))
  (set `self.RefMatch3` (`|GetArrayItem` _outactors)))

(event `self.K2_PostLogin`
  (params (NewPlayer :type "PlayerController Object Reference"))
  (set `self.New Player` NewPlayer)
  (`self.RestartPlayer` null))

(event `self.K2_OnRestartPlayer`
  (params (NewPlayer :type "Controller Object Reference"))
  (add `self.OnDestroyed` (`Controller.K2_GetPawn` NewPlayer) (delegate `PlayerDied`)))

(event `PlayerDied` :!signature `self.OnDestroyed`
  (params (DestroyedActor :type "Actor Object Reference"))
  (`self.RestartPlayer` (`self.New Player`)))

(fn `UserConstructionScript`)